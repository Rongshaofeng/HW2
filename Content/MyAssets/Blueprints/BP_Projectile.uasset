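; BP_Projectile is a projectile actor that reacts when its SphereCollision component hits something.
; On hit it calls ApplyPointDamage with a fixed damage and the reversed velocity direction, though no damaged actor is passed.
; It pushes the struck component with a velocity-scaled impulse at the projectile's location.
; It then spawns an explosion particle effect there and destroys itself.
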(event `self.SphereCollision.OnComponentHit`
  (params (HitComponent :type "PrimitiveComponent Object Reference") (OtherActor :type "Actor Object Reference") (OtherComp :type "PrimitiveComponent Object Reference") (NormalImpulse :type "Vector Structure") (Hit :type "HitResult Structure (by ref)"))
  (`GameplayStatics.ApplyPointDamage` null 30.0 (* (`KismetMathLibrary.Normal` (`self.GetVelocity`)) -1.0) Hit)
  (`PrimitiveComponent.AddImpulseAtLocation` OtherComp (* (`self.GetVelocity`) 10.0) (`self.K2_GetActorLocation`) "None")
  (`/Engine/EditorBlueprintResources/StandardMacros.IsValid` self
    (:`Is Valid`
      (`GameplayStatics.SpawnEmitterAtLocation` "/Game/MobileStarterContent/Particles/P_Explosion.P_Explosion" (`self.K2_GetActorLocation`))
      (`self.K2_DestroyActor`))))

(fn `UserConstructionScript`)